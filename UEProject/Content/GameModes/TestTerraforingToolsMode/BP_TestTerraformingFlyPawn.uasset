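; Test fly pawn for trying out terraforming tools on a CTerraforma landscape, moved by adding physics velocity to its sphere, with right-mouse look.
; A widget selects the Clear, Flat, Up, Down or off tool, setting brush color and zone visibility.
; Each tick it traces the cursor onto the landscape to place the brush.
; Holding left mouse applies the tool there, forces a zone update and resamples the working height.
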(event `self.ReceiveBeginPlay`
  (`|ExecutionSequence`
    (:`then_0`
      (bind _outactors (`GameplayStatics.GetAllActorsOfClass` "/Script/Terraforma.cTerraformaLandscapeActor"))
      (if (> (`KismetArrayLibrary.Array_Length` _outactors) 0)
        (bind _output (`|GetArrayItem` _outactors))
        (set `self.LandscapeComponent` (`self.GetComponentByClass` _output "/Script/Terraforma.cTerraformaLandscapeComponent"))
        (set `self.ZoneComponent` (`self.GetComponentByClass` _output "/Script/Terraforma.cTerraformaZoneComponent"))))
    (:`then_2`
      (set `PlayerController.bShowMouseCursor` true (`GameplayStatics.GetPlayerController` 0))
      (bind _returnvalue (`|CreateWidget` "/Game/GameModes/TestTerraforingToolsMode/W_TerraformingTools.W_TerraformingTools_C"))
      (bind _output_get (set `self.ToolsWidget` _returnvalue))
      (`UserWidget.AddToViewport` _output_get 0)
      (add `/Game/GameModes/TestTerraforingToolsMode/W_TerraformingTools.ChangeToolEventDispatcher` _output_get (delegate `OnSetNewTerraformingTool`))
      (bind _returnvalue_2 (`PrimitiveComponent.CreateDynamicMaterialInstance` (`self.TerraformingToolMesh`) 0 null))
      (set `self.ToolMaterial` _returnvalue_2))))

(event `OnSetNewTerraformingTool`
  (params (NewTool :type "ETerraformingToolEnum Enum"))
  (bind _output_get (set `self.CurrentTerraformingTool` NewTool))
  (`SceneComponent.SetVisibility` (`self.ZoneComponent`) (`|EnumInequality` _output_get "TTE_OFF") false)
  (`MaterialInstanceDynamic.SetVectorParameterValue` (`self.ToolMaterial`) "Color" (select `ETerraformingToolEnum` (`self.CurrentTerraformingTool`) :`TTE_CLEAR` (struct :`R` 1.0 :`B` 0.478672 :`A` 1.0) :`TTE_FLAT` (struct :`R` 1.0 :`G` 1.0 :`B` 1.0 :`A` 1.0) :`TTE_UP` (struct :`G` 1.0 :`A` 1.0) :`TTE_DOWN` (struct :`B` 1.0 :`A` 1.0) :!type "LinearColor Structure")))

(event `InputAxis|TestFlyMoveForward`
  (params (AxisValue :type "Float (single-precision)"))
  (`PrimitiveComponent.SetPhysicsLinearVelocity` (`self.Sphere`) (* (`KismetMathLibrary.GetForwardVector` (`self.GetControlRotation`)) (* AxisValue 1000.0)) true "None"))

(event `InputAxis|TestFlyYaw`
  (params (AxisValue :type "Float (single-precision)"))
  (if (`self.MouseView`)
    (`self.AddControllerYawInput` AxisValue)))

(event `InputAxis|TestFlyMoveRight`
  (params (AxisValue :type "Float (single-precision)"))
  (`PrimitiveComponent.SetPhysicsLinearVelocity` (`self.Sphere`) (* (`KismetMathLibrary.GetRightVector` (`self.GetControlRotation`)) (* AxisValue 500.0)) true "None"))

(event `Key|RightMouseButton`
  (params (Key :type "Key Structure" :default "AnyKey"))
  (bind _returnvalue (`GameplayStatics.GetPlayerController` 0))
  (:`Pressed`
    (set `self.MouseView` true)
    (set `PlayerController.bShowMouseCursor` false _returnvalue))
  (:`Released`
    (set `self.MouseView` false)
    (set `PlayerController.bShowMouseCursor` true _returnvalue)))

(event `InputAxis|TestFlyPitch`
  (params (AxisValue :type "Float (single-precision)"))
  (if (`self.MouseView`)
    (`self.AddControllerPitchInput` AxisValue)))

(event `Key|LeftMouseButton`
  (params (Key :type "Key Structure" :default "AnyKey"))
  (bind (_mouseonlandpos_x _mouseonlandpos_y _mouseonlandpos_z) (`KismetMathLibrary.BreakVector` (`self.MouseOnLandPos`)))
  (:`Pressed`
    (set `self.LeftPressed` true)
    (bind _output_get (set `self.StartTerraformingHeight` (`cTerraformaLandscapeComponent.GetToolHeight` (`self.LandscapeComponent`) (`self.MouseOnLandPos`))))
    (if (< _output_get 1.0)
      (set `self.StartTerraformingHeight` _mouseonlandpos_z)))
  (:`Released`
    (set `self.LeftPressed` false)))

(event `self.ReceiveTick`
  (params (DeltaSeconds :type "Float (single-precision)"))
  (bind (_mouseonlandpos_x _mouseonlandpos_y _mouseonlandpos_z) (`KismetMathLibrary.BreakVector` (`self.MouseOnLandPos`)))
  (bind _startterraformingheight (`self.StartTerraformingHeight`))
  (bind _returnvalue (`KismetMathLibrary.MakeVector` _mouseonlandpos_x _mouseonlandpos_y (select `ETerraformingToolEnum` (`self.CurrentTerraformingTool`) :`TTE_CLEAR` _mouseonlandpos_z :`TTE_FLAT` _startterraformingheight :`TTE_UP` _startterraformingheight :`TTE_DOWN` _startterraformingheight)))
  (bind _returnvalue_2 (and (`self.MouseOnLand`) (`|EnumInequality` (`self.CurrentTerraformingTool`) "TTE_OFF")))
  (`self.UpdateMousePos`)
  (`SceneComponent.SetVisibility` (`self.TerraformingToolMesh`) _returnvalue_2 false)
  (if _returnvalue_2
    (`SceneComponent.K2_SetWorldLocation` (`self.TerraformingToolMesh`) (`self.MouseOnLandPos`) false true)
    (if (`self.LeftPressed`)
      (`cTerraformaLandscapeComponent.ApplyTerraformingTaskTool` (`self.LandscapeComponent`) _returnvalue 800.0 DeltaSeconds (`self.CurrentTerraformingTool`))
      (`cTerraformaZoneComponent.ForceZoneUpdate` (`self.ZoneComponent`))
      (`self.UpdateStartHeight`)
      (`SceneComponent.K2_SetWorldLocation` (`self.TerraformingToolMesh`) _returnvalue false true))))

(fn `UpdateMousePos`
  (bind (_worldlocation _worlddirection) (`PlayerController.DeprojectMousePositionToWorld` (`GameplayStatics.GetPlayerController` 0)))
  (bind (_intersectionlocation _returnvalue) (`cTerraformaLandscapeComponent.LineIntersection` (`self.LandscapeComponent`) _worldlocation (* _worlddirection 1000000.0)))
  (bind _output_get (set `self.MouseOnLand` _returnvalue))
  (if _output_get
    (set `self.MouseOnLandPos` _intersectionlocation)))

(fn `UpdateStartHeight`
  (set `self.StartTerraformingHeight` (`cTerraformaLandscapeComponent.GetToolHeight` (`self.LandscapeComponent`) (`self.MouseOnLandPos`))))

(fn `UserConstructionScript`)