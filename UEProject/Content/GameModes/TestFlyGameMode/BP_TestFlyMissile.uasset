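; Missile actor for the test fly game mode that blasts a painted crater into Terraforma landscape on impact.
; On BeginPlay it finds the landscape's terraform component and builds cut, height and color templates from textures.
; Each Tick it moves by its velocity without sweep, testing that step with the component's own line intersection.
; On a hit it destroys itself, applies the templates within a vertical band and spawns an enlarged explosion.
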(event `self.ReceiveBeginPlay`
  (`|ExecutionSequence`
    (:`then_0`
      (bind _outactors (`GameplayStatics.GetAllActorsOfClass` "/Script/Terraforma.cTerraformaLandscapeActor"))
      (if (> (`KismetArrayLibrary.Array_Length` _outactors) 0)
        (set `self.LandscapeComponent` (`self.GetComponentByClass` (`|GetArrayItem` _outactors) "/Script/Terraforma.cTerraformaLandscapeComponent"))))
    (:`then_1`
      (set `self.BombTemplateCutH` (`cTerraformaUtilsLibrary.GetHeightMapTemplateFromTexture` (`self.BombTemplateHeightmap2`)))
      (set `self.BombTemplateH` (`cTerraformaUtilsLibrary.GetHeightMapTemplateFromTexture` (`self.BombTemplateHeightmap`)))
      (set `self.BombTemplateColor` (`cTerraformaUtilsLibrary.GetColorMapTemplateFromTexture` (`self.BombTemplateTexture`))))))

(event `self.ReceiveTick`
  (params (DeltaSeconds :type "Float (single-precision)"))
  (bind _returnvalue (* (`self.Speed`) DeltaSeconds))
  (bind _output_get (set `self.PrevPos` (`self.K2_GetActorLocation`)))
  (bind _output_get_2 (set `self.CurrentPos` (+ _returnvalue _output_get)))
  (`self.K2_SetActorLocation` _output_get_2 false true)
  (bind (_intersectionlocation _returnvalue_2) (`cTerraformaLandscapeComponent.LineIntersection` (`self.LandscapeComponent`) _output_get _returnvalue))
  (if _returnvalue_2
    (`self.K2_DestroyActor`)
    (bind _z (.z _intersectionlocation))
    (`cTerraformaLandscapeComponent.ApplyTerraforming` (`self.LandscapeComponent`) _intersectionlocation (`self.BombTemplateCutH`) (`self.BombTemplateH`) 7 (`self.BombTemplateColor`) (- _z 200.0) (+ _z 200.0))
    (bind _returnvalue_3 (`GameplayStatics.SpawnEmitterAtLocation` "/Game/StarterContent/Particles/P_SmallExplosion.P_SmallExplosion" _intersectionlocation))
    (`SceneComponent.SetWorldScale3D` _returnvalue_3 (4.0 4.0 4.0))))

(fn `UserConstructionScript`)