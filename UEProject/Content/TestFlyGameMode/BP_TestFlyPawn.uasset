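; Test pawn for flying over a Terraforma landscape and editing it with the mouse.
; Input axes add velocity to a physics sphere along the view, and holding right mouse enables look.
; Holding left mouse applies one of two texture-derived heightmap templates at intervals on Tick, with Left Ctrl selecting the second.
; UpdateMousePos intersects the cursor ray with the landscape component, also placing the falling missile that middle mouse spawns.
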(event `self.ReceiveBeginPlay`
  (`|ExecutionSequence`
    (:`then_0`
      (bind _outactors (`GameplayStatics.GetAllActorsOfClass` "/Script/Terraforma.cTerraformaLandscapeActor"))
      (if (> (`KismetArrayLibrary.Array_Length` _outactors) 0)
        (set `self.LandscapeComponent` (`self.GetComponentByClass` (`|GetArrayItem` _outactors) "/Script/Terraforma.cTerraformaLandscapeComponent"))))
    (:`then_1`
      (set `self.TerraforminTemplate1Heigthmap` (`cTerraformaUtilsLibrary.GetHeightMapTemplateFromTexture` (`self.TerraformingTemplate1`)))
      (set `self.TerraforminTemplate2Heigthmap` (`cTerraformaUtilsLibrary.GetHeightMapTemplateFromTexture` (`self.TerraformingTemplate2`))))
    (:`then_2`
      (set `PlayerController.bShowMouseCursor` true (`GameplayStatics.GetPlayerController` 0)))))

(event `InputAxis|TestFlyMoveForward`
  (params (AxisValue :type "Float (single-precision)"))
  (`PrimitiveComponent.SetPhysicsLinearVelocity` (`self.Sphere`) (* (`KismetMathLibrary.GetForwardVector` (`self.GetControlRotation`)) (* AxisValue 1000.0)) true "None"))

(event `InputAxis|TestFlyYaw`
  (params (AxisValue :type "Float (single-precision)"))
  (if (`self.MouseView`)
    (`self.AddControllerYawInput` AxisValue)))

(event `InputAxis|TestFlyMoveRight`
  (params (AxisValue :type "Float (single-precision)"))
  (`PrimitiveComponent.SetPhysicsLinearVelocity` (`self.Sphere`) (* (`KismetMathLibrary.GetRightVector` (`self.GetControlRotation`)) (* AxisValue 500.0)) true "None"))

(event `InputAxis|TestFlyPitch`
  (params (AxisValue :type "Float (single-precision)"))
  (if (`self.MouseView`)
    (`self.AddControllerPitchInput` AxisValue)))

(event `Key|RightMouseButton`
  (params (Key :type "Key Structure" :default "AnyKey"))
  (bind _returnvalue (`GameplayStatics.GetPlayerController` 0))
  (:`Pressed`
    (set `self.MouseView` true)
    (set `PlayerController.bShowMouseCursor` false _returnvalue))
  (:`Released`
    (set `self.MouseView` false)
    (set `PlayerController.bShowMouseCursor` true _returnvalue)))

(event `Key|LeftControl`
  (params (Key :type "Key Structure" :default "AnyKey"))
  (:`Pressed`
    (set `self.CtrlPressed` true))
  (:`Released`
    (set `self.CtrlPressed` false)))

(event `Key|LeftMouseButton`
  (params (Key :type "Key Structure" :default "AnyKey"))
  (:`Pressed`
    (set `self.Terraforming` true))
  (:`Released`
    (set `self.Terraforming` false)))

(event `Key|MiddleMouseButton`
  (params (Key :type "Key Structure" :default "AnyKey"))
  (:`Pressed`
    (`self.UpdateMousePos`)
    (bind _returnvalue (`|SpawnActorFromClass` "/Game/TestFlyGameMode/BP_TestFlyMissile.BP_TestFlyMissile_C" (`KismetMathLibrary.MakeTransform` (+ (`self.MouseOnLandPos`) (0.0 0.0 1700.0))) "AlwaysSpawn" "OverrideRootScale"))
    (set `/Game/TestFlyGameMode/BP_TestFlyMissile.Speed` (0.0 0.0 -400.0) _returnvalue)))

(event `self.ReceiveTick`
  (params (DeltaSeconds :type "Float (single-precision)"))
  (bind _returnvalue (+ (`self.TerraformingTime`) DeltaSeconds))
  (`|ExecutionSequence`
    (:`then_0`
      (if (`self.Terraforming`)
        (`self.UpdateMousePos`)))
    (:`then_1`
      (if (and (`self.Terraforming`) (`self.MouseOnLand`))
        (if (>= _returnvalue (`self.TERRAFORMING_DELAY`))
          (set `self.TerraformingTime` 0.0)
          (if (`self.CtrlPressed`)
            (`cTerraformaLandscapeComponent.ApplyTerraforming` (`self.LandscapeComponent`) (`self.MouseOnLandPos`) (make `sTerraformaTemplate`) (`self.TerraforminTemplate2Heigthmap`) 5 (make `sTerraformaTemplate`) 0.0 6400.0)
            (else
              (`cTerraformaLandscapeComponent.ApplyTerraforming` (`self.LandscapeComponent`) (`self.MouseOnLandPos`) (make `sTerraformaTemplate`) (`self.TerraforminTemplate1Heigthmap`) 5 (make `sTerraformaTemplate`) 0.0 6400.0)))
          (else
            (set `self.TerraformingTime` _returnvalue)))))))

(fn `UpdateMousePos`
  (bind (_worldlocation _worlddirection) (`PlayerController.DeprojectMousePositionToWorld` (`GameplayStatics.GetPlayerController` 0)))
  (bind (_intersectionlocation _returnvalue) (`cTerraformaLandscapeComponent.LineIntersection` (`self.LandscapeComponent`) _worldlocation (* _worlddirection 1000000.0)))
  (bind _output_get (set `self.MouseOnLand` _returnvalue))
  (if _output_get
    (set `self.MouseOnLandPos` _intersectionlocation)))

(fn `UserConstructionScript`)